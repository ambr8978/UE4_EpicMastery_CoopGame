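; BP_AdvancedAI is an AI-controlled actor that runs the BT_AdvancedAI behavior tree through its AI controller on BeginPlay.
; A separate function writes player pawn 0 into the blackboard's TargetActor key, though nothing in this Blueprint calls it.
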(event EventBeginPlay
  (CallFunction|SetupandRunBehaviourTree))

(fn ConstructionScript)

(fn SetupandRunBehaviourTree
  (AI|RunBehaviorTree (AI|GetAIController self) "/Game/AdvancedAI/BT_AdvancedAI.BT_AdvancedAI"))

(fn SetTargetActorBlackboardValue
  (AI|Components|Blackboard|SetValueasObject (AI|GetBlackboard self) (Utilities|Name|MakeLiteralName "TargetActor") (Game|Player|GetPlayerPawn 0)))