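; Grenade projectile actor that explodes on a short fixed fuse after BeginPlay, with no impact trigger in its graphs.
; Explode spawns the explosion particle, applies full radial damage without falloff inside DamageRadius, and destroys the actor.
; Damage is credited to the instigator's controller, and a debug sphere briefly shows the blast radius.
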(event Custom|Explode
  (Effects|SpawnEmitteratLocation "/Game/WeaponEffects/Explosion/P_Explosion.P_Explosion" (Transformation|GetActorLocation))
  (Game|Damage|ApplyRadialDamage 1e+02 (Transformation|GetActorLocation) (Variables|Default|GetDamageRadius) 0 0 self (Game|GetInstigatorController) true "ECC_Visibility")
  (Actor|DestroyActor)
  (Rendering|Debug|DrawDebugSphere (Transformation|GetActorLocation) (Variables|Default|GetDamageRadius) 12 "(R=1.000000,G=0.750629,B=0.064417,A=1.000000)" 1.0 3.0))

(event EventBeginPlay
  (Utilities|FlowControl|Delay 1.0)
  (CallFunction|Explode))

(fn ConstructionScript)